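; AI character that acts as a shootable target, awarding the player a point when a projectile hits it.
; BeginPlay caches the first player's BP_PlayerCharacter as a reference.
; When a Projectile begins overlapping the CollisionBox, it increments that character's Points, then destroys both itself and the projectile.
; The file holds no movement or decision logic, and the construction script is empty.
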(event OnComponentBeginOverlap(CollisionBox)
  (params (OverlappedComponent :type Primitive%20Component%20Object%20Reference) (OtherActor :type Actor%20Object%20Reference) (OtherComp :type Primitive%20Component%20Object%20Reference) (OtherBodyIndex :type Integer) (bFromSweep :type Boolean) (SweepResult :type Hit%20Result%20Structure%20%28by%20ref%29))
  (bind _char_ref (Variables|Default|GetChar%20Ref))
  (Utilities|Casting|CastToProjectile OtherActor)
  (Variables|/Game/Blueprints/BP_PlayerCharacter.BP_PlayerCharacter_C|SetPoints _char_ref (+ (Variables|/Game/Blueprints/BP_PlayerCharacter.BP_PlayerCharacter_C|GetPoints _char_ref) 1))
  (Actor|DestroyActor)
  (Actor|DestroyActor OtherActor))

(event EventBeginPlay
  (bind _asbp_player_character (Utilities|Casting|CastToBP_PlayerCharacter (Game|GetPlayerCharacter 0)))
  (Variables|Default|SetChar%20Ref _asbp_player_character))

(fn ConstructionScript)