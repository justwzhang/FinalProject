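; BP_PlayerCharacter is a player character that tracks wave-based growth values and opens a wave screen when the score target is reached.
; Each Tick recomputes log N, N, N log N and N squared from WaveNum, mirroring Big-O complexity classes.
; It then checks Points against TargetScore and, once met, creates Wave_Widget, shows the mouse cursor and pauses the game.
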(event EventBeginPlay)

(event Collision|EventActorBeginOverlap
  (params (OtherActor :type Actor%20Object%20Reference)))

(event EventTick
  (params (DeltaSeconds :type Float%20%28single-precision%29))
  (Utilities|FlowControl|Sequence
    (:then_0
      (Variables|Default|SetO%28log%20n%29_Value (Math|Float|Ceil (Math|Float|Loge (Math|Conversions|ToFloat(Integer) (Variables|Default|GetWave_Num)))))
      (Variables|Default|SetO%28n%29_Value (Variables|Default|GetWave_Num))
      (Variables|Default|SetO%28n%20log%20n%29_Value (Math|Float|Ceil (* (Variables|Default|GetWave_Num) (Math|Float|Loge (Math|Conversions|ToFloat(Integer) (Variables|Default|GetWave_Num))))))
      (Variables|Default|SetO%28n^2%29_Value (* (Variables|Default|GetWave_Num) (Variables|Default|GetWave_Num))))
    (:then_1
      (if (>= (Variables|Default|GetPoints) (Variables|Default|GetTarget%20Score))
        (bind _returnvalue (UserInterface|CreateWidget "/Game/Blueprints/Wave_Widget.Wave_Widget_C"))
        (UserInterface|Viewport|AddtoViewport _returnvalue 0)
        (Variables|/Script/Engine.PlayerController|SetbShowMouseCursor (Game|GetPlayerController 0) true)
        (Game|SetGamePaused true)))))

(fn ConstructionScript)