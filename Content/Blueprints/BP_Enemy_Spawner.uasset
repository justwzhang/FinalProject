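; BP_Enemy_Spawner spawns BP_AICharacter enemies periodically while the player's Points are short of TargetScore.
; Tick caches the player character and runs through a Delay of SpawnDelay, which paces the spawns.
; Player Option values 1 to 5 all lead to the same single-enemy SpawnEnemy call.
; SpawnEnemy spawns only while the player's NumToSpawn is above zero, decrementing that shared budget each time.
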(event Custom|Spawn%20Enemy
  (params (Enemy :type Actor%20Class%20Reference) (SpawnTransform :type Transform) (Num%20Enemies :type Integer))
  (bind _char_ref (Variables|Default|GetChar%20Ref))
  (if (> (Variables|/Game/Blueprints/BP_PlayerCharacter.BP_PlayerCharacter_C|GetNumToSpawn _char_ref) 0)
    (Variables|/Game/Blueprints/BP_PlayerCharacter.BP_PlayerCharacter_C|SetNumToSpawn _char_ref (- (Variables|/Game/Blueprints/BP_PlayerCharacter.BP_PlayerCharacter_C|GetNumToSpawn _char_ref) 1))
    (Game|SpawnActorfromClass Enemy SpawnTransform "Undefined" 0 0)))

(event EventTick
  (params (DeltaSeconds :type Float%20%28single-precision%29))
  (bind _asbp_player_character (Utilities|Casting|CastToBP_PlayerCharacter (Game|GetPlayerCharacter 0)))
  (Variables|Default|SetChar%20Ref _asbp_player_character)
  (if (>= (- (Variables|/Game/Blueprints/BP_PlayerCharacter.BP_PlayerCharacter_C|GetTarget%20Score (Variables|Default|GetChar%20Ref)) (Variables|/Game/Blueprints/BP_PlayerCharacter.BP_PlayerCharacter_C|GetPoints (Variables|Default|GetChar%20Ref))) 1)
    (Utilities|FlowControl|Delay (Variables|Default|GetSpawn%20Delay))
    (Utilities|FlowControl|Sequence
      (:then_0
        (if (== (Variables|/Game/Blueprints/BP_PlayerCharacter.BP_PlayerCharacter_C|GetOption (Variables|Default|GetChar%20Ref)) 1)
          (CallFunction|SpawnEnemy :Enemy "/Game/Blueprints/BP_AICharacter.BP_AICharacter_C" :Num%20Enemies 1 :!label _label)))
      (:then_1
        (if (== (Variables|/Game/Blueprints/BP_PlayerCharacter.BP_PlayerCharacter_C|GetOption (Variables|Default|GetChar%20Ref)) 2)
          (goto _label)))
      (:then_2
        (if (== (Variables|/Game/Blueprints/BP_PlayerCharacter.BP_PlayerCharacter_C|GetOption (Variables|Default|GetChar%20Ref)) 3)
          (goto _label)))
      (:then_3
        (if (== (Variables|/Game/Blueprints/BP_PlayerCharacter.BP_PlayerCharacter_C|GetOption (Variables|Default|GetChar%20Ref)) 4)
          (goto _label)))
      (:then_4
        (if (== (Variables|/Game/Blueprints/BP_PlayerCharacter.BP_PlayerCharacter_C|GetOption (Variables|Default|GetChar%20Ref)) 5)
          (goto _label))))))

(fn ConstructionScript)